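; Checkpoint actor that lets the player save progress by pressing E inside a cylinder trigger, which is hidden at BeginPlay.
; Overlap by BP_ThirdPersonCharacterCustom enables the actor's input and shows W_InteractSave; leaving disables input and removes the prompt.
; E calls SaveCheckpoint on the character reference from the end-overlap cast, plays the Checkpoint sound and shows W_Saving for one second.
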(event `self.ReceiveBeginPlay`
  (`SceneComponent.SetVisibility` (`self.Cylinder`) false false))

(event `self.Cylinder.OnComponentBeginOverlap`
  (params (OverlappedComponent :type "PrimitiveComponent Object Reference") (OtherActor :type "Actor Object Reference") (OtherComp :type "PrimitiveComponent Object Reference") (OtherBodyIndex :type Integer) (bFromSweep :type Boolean) (SweepResult :type "HitResult Structure (by ref)"))
  (cast `/Game/Blueprints/BP_ThirdPersonCharacterCustom` OtherActor)
  (`self.EnableInput` (`GameplayStatics.GetPlayerController` 0))
  (bind _returnvalue (`|CreateWidget` "/Game/Widgets/W_InteractSave.W_InteractSave_C"))
  (`UserWidget.AddToViewport` _returnvalue 0))

(event `self.Cylinder.OnComponentEndOverlap`
  (params (OverlappedComponent :type "PrimitiveComponent Object Reference") (OtherActor :type "Actor Object Reference") (OtherComp :type "PrimitiveComponent Object Reference") (OtherBodyIndex :type Integer))
  (bind _asbp_third_person_character_custom (cast `/Game/Blueprints/BP_ThirdPersonCharacterCustom` OtherActor))
  (`self.DisableInput` null)
  (`Widget.RemoveFromParent` (stale `self.Cylinder.OnComponentBeginOverlap` _returnvalue)))

(event `Key|E`
  (params (Key :type "Key Structure"))
  (:`Pressed`
    (`/Game/Blueprints/BP_ThirdPersonCharacterCustom.Save Checkpoint` (stale `self.Cylinder.OnComponentEndOverlap` _asbp_third_person_character_custom))
    (`GameplayStatics.PlaySoundAtLocation` "/Game/Sounds/Checkpoint.Checkpoint" (`SceneComponent.K2_GetComponentLocation` (`self.Cylinder`)) (struct) 1.0 1.0 0.0 null null null null)
    (bind _returnvalue (`|CreateWidget` "/Game/Widgets/W_Saving.W_Saving_C"))
    (`UserWidget.AddToViewport` _returnvalue 0)
    (`KismetSystemLibrary.Delay` 1.0)
    (`Widget.RemoveFromParent` _returnvalue)))

(fn `UserConstructionScript`)