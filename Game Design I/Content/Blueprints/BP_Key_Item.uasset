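; BP_Key_Item is a key pickup that the player carries to unlock locked doors.
; Overlapping its box asks the custom third-person character to pick it up, increments that character's key count and plays a jangle.
; Overlapping a BP_Door_Locked clears its locked flag, plays an unlock sound and destroys the key.
; Pickup attaches the cylinder to the hand_r socket without collision, while Drop detaches it and restores collision with simulated physics.
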(event `self.ReceiveBeginPlay`
  (`KismetSystemLibrary.PrintString` "This Key Exists!" true true (struct :`R` 0.989389 :`G` 0.130208 :`B` 1.0 :`A` 1.0)))

(event `self.BoxCollision.OnComponentBeginOverlap`
  (params (OverlappedComponent :type "PrimitiveComponent Object Reference") (OtherActor :type "Actor Object Reference") (OtherComp :type "PrimitiveComponent Object Reference") (OtherBodyIndex :type Integer) (bFromSweep :type Boolean) (SweepResult :type "HitResult Structure (by ref)"))
  (`|ExecutionSequence`
    (:`then_0`
      (bind _asbp_third_person_character_custom (cast `/Game/Blueprints/BP_ThirdPersonCharacterCustom` OtherActor)
        (:`then`
          (`/Game/Blueprints/BP_ThirdPersonCharacterCustom.TryToPickUp` _asbp_third_person_character_custom self)
          ;[1 1 1] Key Counter
          (`KismetSystemLibrary.PrintString` "Key has been Overlapped by Player" true true (struct :`G` 0.66 :`B` 1.0 :`A` 1.0) 5.0)
          (bind _key_count (`/Game/Blueprints/BP_ThirdPersonCharacterCustom.Key Count` _asbp_third_person_character_custom))
          (set `/Game/Blueprints/BP_ThirdPersonCharacterCustom.Key Count` (+ _key_count 1) _asbp_third_person_character_custom) ; Set Key Count
          (`KismetSystemLibrary.PrintString` (`KismetStringLibrary.Concat_StrStr` "The Player has " (`KismetStringLibrary.Conv_IntToString` _key_count) " key(s)."))
          (`GameplayStatics.PlaySoundAtLocation` "/Game/Sounds/KeyJangle.KeyJangle" (`SceneComponent.K2_GetComponentLocation` (`self.BoxCollision`)) (struct) 1.0 1.0 0.0 null null null null))
        (:`CastFailed`
          (`KismetSystemLibrary.PrintString` "Key Player Cast Failed" true true (struct :`R` 0.875 :`B` 0.029306 :`A` 1.0)))))
    (:`then_1`
      (bind _asbp_door_locked (cast `/Game/Blueprints/BP_Door_Locked` OtherActor)
        (:`then`
          (set `/Game/Blueprints/BP_Door.IsLocked` false _asbp_door_locked)
          (`GameplayStatics.PlaySoundAtLocation` "/Game/Sounds/Unlock.Unlock" (`SceneComponent.K2_GetComponentLocation` (`self.Cylinder`)) (struct) 1.0 1.0 0.0 null null null null)
          (`self.K2_DestroyActor`))
        (:`CastFailed`
          (`KismetSystemLibrary.PrintString` "There was an Error"))))))

(event `/Game/Blueprints/BPI_Item.Pickup`
  (params (ParentMesh :type "SkeletalMeshComponent Object Reference"))
  (`SceneComponent.K2_AttachToComponent` (`self.Cylinder`) ParentMesh "hand_r" "SnapToTarget" "KeepRelative" "KeepRelative" true)
  (`PrimitiveComponent.SetCollisionEnabled` (`self.Cylinder`) "NoCollision") ; Collide with the ground please
)

(event `/Game/Blueprints/BPI_Item.Drop`
  (bind _cylinder (`self.Cylinder`))
  (set `self.Drop Location` (`SceneComponent.K2_GetComponentLocation` _cylinder))
  (`SceneComponent.K2_DetachFromComponent` _cylinder "KeepRelative" "KeepRelative" "KeepRelative" true) ; Don't follow the hand anymore
  (`PrimitiveComponent.SetSimulatePhysics` (`self.Cylinder`) true) ; use gravity to fall
  (`PrimitiveComponent.SetCollisionEnabled` (`self.Cylinder`) "QueryAndPhysics") ; Collide with the ground please
  (`SceneComponent.K2_SetWorldLocation` (`self.Cylinder`) (`self.Drop Location`) false false) ; To prevent the can from going to world origin
)

(fn `UserConstructionScript`
  (`parent.UserConstructionScript`))