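; BP_Cabinet is an interactable cabinet whose two doors swing open when the player presses E nearby.
; Overlapping InteractCollision with BP_ThirdPersonCharacterCustom enables input and shows a W_Interact prompt; leaving reverses both.
; E plays a Timeline that lerps the door yaws in opposite directions.
; An IsShut flag blocks re-triggering until a Delay in the Timeline update resets it, though no closing animation exists.
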(event `self.InteractCollision.OnComponentBeginOverlap`
  (params (OverlappedComponent :type "PrimitiveComponent Object Reference") (OtherActor :type "Actor Object Reference") (OtherComp :type "PrimitiveComponent Object Reference") (OtherBodyIndex :type Integer) (bFromSweep :type Boolean) (SweepResult :type "HitResult Structure (by ref)"))
  (cast `/Game/Blueprints/BP_ThirdPersonCharacterCustom` OtherActor)
  (`self.EnableInput` (`GameplayStatics.GetPlayerController` 0))
  (bind _returnvalue (`|CreateWidget` "/Game/Widgets/W_Interact.W_Interact_C"))
  (`UserWidget.AddToViewport` _returnvalue 0))

(event `self.InteractCollision.OnComponentEndOverlap`
  (params (OverlappedComponent :type "PrimitiveComponent Object Reference") (OtherActor :type "Actor Object Reference") (OtherComp :type "PrimitiveComponent Object Reference") (OtherBodyIndex :type Integer))
  (cast `/Game/Blueprints/BP_ThirdPersonCharacterCustom` OtherActor)
  (`self.DisableInput` null)
  (`Widget.RemoveFromParent` (stale `self.InteractCollision.OnComponentBeginOverlap` _returnvalue)))

(event `Key|E`
  (params (Key :type "Key Structure"))
  (:`Pressed`
    (if (`self.IsShut`)
      (`self.DoorOpen`)
      (else
        (`KismetSystemLibrary.PrintString` "Cabinet is Open")))))

(event `self.ReceiveBeginPlay`
  (set `self.IsShut` true))

(event `DoorOpen`
  (bind (_direction _doorfloat) (`Timeline|Timeline` :!via `PlayFromStart`)
    (:`Update`
      (`SceneComponent.K2_SetRelativeRotation` (`self.chinese_cabinet_2k_chinese_cabinet_door_01`) (`KismetMathLibrary.MakeRotator` 0.0 0.0 (`KismetMathLibrary.Lerp` 0.0 120.0 _doorfloat)) false false)
      (`SceneComponent.K2_SetRelativeRotation` (`self.chinese_cabinet_2k_chinese_cabinet_door_02`) (`KismetMathLibrary.MakeRotator` 0.0 0.0 (`KismetMathLibrary.Lerp` 0.0 -120.0 _doorfloat)) false false)
      (set `self.IsShut` false)
      (`KismetSystemLibrary.Delay` 3.0)
      (set `self.IsShut` true))))

(fn `UserConstructionScript`)