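; BP_Book is an interactable book actor that shows an info screen when the player uses it.
; Overlapping its InteractCollision with the custom third-person character enables input on the book and shows a W_Interact prompt widget; leaving disables input and removes the prompt.
; While input is enabled, pressing E creates and displays a W_BookInfo widget, which this Blueprint never removes.
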(event `self.InteractCollision.OnComponentBeginOverlap`
  (params (OverlappedComponent :type "PrimitiveComponent Object Reference") (OtherActor :type "Actor Object Reference") (OtherComp :type "PrimitiveComponent Object Reference") (OtherBodyIndex :type Integer) (bFromSweep :type Boolean) (SweepResult :type "HitResult Structure (by ref)"))
  (cast `/Game/Blueprints/BP_ThirdPersonCharacterCustom` OtherActor)
  (`self.EnableInput` (`GameplayStatics.GetPlayerController` 0))
  (bind _returnvalue (`|CreateWidget` "/Game/Widgets/W_Interact.W_Interact_C"))
  (`UserWidget.AddToViewport` _returnvalue 0))

(event `self.InteractCollision.OnComponentEndOverlap`
  (params (OverlappedComponent :type "PrimitiveComponent Object Reference") (OtherActor :type "Actor Object Reference") (OtherComp :type "PrimitiveComponent Object Reference") (OtherBodyIndex :type Integer))
  (cast `/Game/Blueprints/BP_ThirdPersonCharacterCustom` OtherActor)
  (`self.DisableInput` null)
  (`Widget.RemoveFromParent` (stale `self.InteractCollision.OnComponentBeginOverlap` _returnvalue)))

(event `Key|E`
  (params (Key :type "Key Structure"))
  (:`Pressed`
    (bind _returnvalue (`|CreateWidget` "/Game/Widgets/W_BookInfo.W_BookInfo_C"))
    (`UserWidget.AddToViewport` _returnvalue 0)))

(fn `UserConstructionScript`
  (`parent.UserConstructionScript`))