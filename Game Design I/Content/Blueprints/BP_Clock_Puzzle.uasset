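; BP_Clock_Puzzle is an interactable puzzle object whose logic is unfinished.
; Actor overlap with BP_ThirdPersonCharacterCustom toggles AbleToInteract, which starts false on BeginPlay.
; Interact prints a move-closer message when out of range and does nothing when in range.
; An unconnected branch, noted as an open question, would cast to BP_MovingShelf and call MoveRight, so the clock does not move any shelf.
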(event `self.ReceiveBeginPlay`
  (set `self.Able to Interact` false))

(event `self.ReceiveActorBeginOverlap`
  (params (OtherActor :type "Actor Object Reference"))
  (cast `/Game/Blueprints/BP_ThirdPersonCharacterCustom` OtherActor)
  (set `self.Able to Interact` true))

(event `self.ReceiveActorEndOverlap`
  (params (OtherActor :type "Actor Object Reference"))
  (cast `/Game/Blueprints/BP_ThirdPersonCharacterCustom` OtherActor)
  (set `self.Able to Interact` false))

(event `/Game/Blueprints/BPI_Puzzle.Interact`
  (if (not (`self.Able to Interact`))
    (`KismetSystemLibrary.PrintString` "Move Closer to Interact with an Object")))

(fn `UserConstructionScript`)