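; A locked door that costs the player character a key to open and later serves as a level exit.
; On box overlap while shut and locked, it spends a key to unlock and open, or prints a warning.
; DoorOpen swings the mesh via a Timeline with a creak, then re-flags it shut after a delay.
; Later overlaps while flagged shut reopen it, fade the camera and open the Destination level.
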(event `self.ReceiveBeginPlay`
  (set `self.IsLocked` true)
  (set `self.IsShut` true))

(event `self.Box collision.OnComponentBeginOverlap`
  (params (OverlappedComponent :type "PrimitiveComponent Object Reference") (OtherActor :type "Actor Object Reference") (OtherComp :type "PrimitiveComponent Object Reference") (OtherBodyIndex :type Integer) (bFromSweep :type Boolean) (SweepResult :type "HitResult Structure (by ref)"))
  (bind _returnvalue (`GameplayStatics.GetPlayerCameraManager` 0))
  (if (`self.IsShut`)
    (if (`self.IsLocked`)
      (bind _asbp_third_person_character_custom (cast `/Game/Blueprints/BP_ThirdPersonCharacterCustom` OtherActor))
      (bind _key_count (`/Game/Blueprints/BP_ThirdPersonCharacterCustom.Key Count` _asbp_third_person_character_custom))
      (if (> _key_count 0)
        (set `self.IsShut` false)
        (set `self.IsLocked` false)
        (set `/Game/Blueprints/BP_ThirdPersonCharacterCustom.Key Count` (- _key_count 1) _asbp_third_person_character_custom) ; Remove a Key, then open door.
        (`|ExecutionSequence`
          (:`then_0`
            (`self.DoorOpen`)))
        (else
          (`KismetSystemLibrary.PrintString` "Get More Keys! Door is locked" true true (struct :`R` 0.479167 :`G` 0.051103 :`A` 1.0) 5.0)))
      (else
        (set `self.IsShut` false)
        (`self.DoorOpen`)
        ;[0.927 0.02966 0.08949] SwapLevel
        (cast `/Game/Blueprints/BP_ThirdPersonCharacterCustom` OtherActor
          (:`then`
            (`self.Destination` ; Convert to Validated Get on Destination
              (:`then`
                (`PlayerCameraManager.StartCameraFade` :`self` _returnvalue :`ToAlpha` 1.0 :`Duration` 1.0 :`bShouldFadeAudio` true)
                (`KismetSystemLibrary.Delay` 1.0)
                (`GameplayStatics.OpenLevelBySoftObjectPtr` (`self.Destination`))
                (`PlayerCameraManager.StartCameraFade` :`self` _returnvalue :`FromAlpha` 1.0 :`Duration` 1.0 :`bShouldFadeAudio` true))
              (:`else`
                (`KismetSystemLibrary.PrintString` "No Valid Destination" true true (struct :`R` 1.0 :`G` 0.041493 :`A` 1.0)))))
          (:`CastFailed`
            (`KismetSystemLibrary.PrintString` "Cast to Open Level Failed" true true (struct :`R` 0.927 :`G` 0.029664 :`B` 0.089486 :`A` 1.0))))))
    (else
      (`KismetSystemLibrary.PrintString` "Door Moving"))))

(event `DoorOpen`
  (`|ExecutionSequence`
    (:`then_0`
      (bind (_direction _doorfloat) (`Timeline|Timeline` :!via `PlayFromStart`)
        (:`Update`
          (`SceneComponent.K2_SetRelativeRotation` (`self.SM_Door`) (`KismetMathLibrary.MakeRotator` 0.0 0.0 (`KismetMathLibrary.Lerp` 0.0 90.0 _doorfloat)) false false)
          (`KismetSystemLibrary.Delay` 7.0)
          (set `self.IsShut` true))))
    (:`then_1`
      (`GameplayStatics.PlaySoundAtLocation` "/Game/Sounds/DoorCreak.DoorCreak" (`SceneComponent.K2_GetComponentLocation` (`self.SM_Door`)) (struct) 1.0 1.0 0.0 null null null null))))

(fn `UserConstructionScript`)