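; BP_PatrolAI is an AI character that endlessly wanders between actors tagged PatrolRoute at a walk speed randomized on BeginPlay.
; It shuffles the gathered points, then MoveToPatrolPoint loops through them with AIMoveTo and a short delay, advancing even on failure and reshuffling after each full pass.
; A similar looping MoveToPlayer event follows the player character, but nothing in this Blueprint calls it.
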(event `self.ReceiveBeginPlay`
  ;[1 1 1] BeginPlay-Start Patrol
  (bind _outactors (`GameplayStatics.GetAllActorsOfClassWithTag` "/Script/Engine.Actor" (`self.PatrolRoute`)))
  (`KismetSystemLibrary.PrintString` (`KismetStringLibrary.Concat_StrStr` "There are " (`KismetStringLibrary.Conv_IntToString` (`KismetArrayLibrary.Array_Length` _outactors)) " this many patrol points."))
  (`KismetArrayLibrary.Array_Shuffle` _outactors)
  (set `CharacterMovementComponent.MaxWalkSpeed` (`KismetMathLibrary.Conv_IntToDouble` (* (`KismetMathLibrary.RandomIntegerInRange` 8 12) 25)) (`self.CharacterMovement`))
  (`self.MoveToPatrolPoint`))

(event `MoveToPatrolPoint`
  ;[1 1 1] Patrol
  (`|AIMoveTo` self (`self.K2_GetActorLocation` (`|GetArrayItem` (stale `self.ReceiveBeginPlay` _outactors) (`self.CurrentPatrolPoint`))) null 0.0 ; Move to the player's location, constantly updating and stopping 2 meters away
    (:`OnSuccess`
      (`KismetSystemLibrary.PrintString` "Successful Move"))
    (:`OnFail`
      (`KismetSystemLibrary.PrintString` "Failed to Get Player" true true (struct :`R` 1.0 :`G` 0.045751 :`B` 0.057688 :`A` 1.0))))
  (bind _result (`/Engine/EditorBlueprintResources/StandardMacros.IncrementInt` (`self.CurrentPatrolPoint`))
    (:`  `
      (if (>= _result (`KismetArrayLibrary.Array_Length` (stale `self.ReceiveBeginPlay` _outactors)))
        (set `self.CurrentPatrolPoint` 0)
        (`KismetArrayLibrary.Array_Shuffle` (stale `self.ReceiveBeginPlay` _outactors)))
      (`KismetSystemLibrary.Delay` 1.0)
      (`self.MoveToPatrolPoint`))))

(event `MoveToPlayer`
  ;[1 1 1] Go to Player
  (`|AIMoveTo` self (0.0 0.0 0.0) (`GameplayStatics.GetPlayerCharacter` 0) 200.0 ; Move to the player's location, constantly updating and stopping 2 meters away
    (:`OnSuccess`
      (`KismetSystemLibrary.PrintString` "Successful Move"))
    (:`OnFail`
      (`KismetSystemLibrary.PrintString` "Failed to Get Player" true true (struct :`R` 1.0 :`G` 0.045751 :`B` 0.057688 :`A` 1.0))))
  (`KismetSystemLibrary.Delay` 1.0)
  (`self.MoveToPlayer`))

(fn `UserConstructionScript`)